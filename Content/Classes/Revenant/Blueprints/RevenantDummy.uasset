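; RevenantDummy is a dummy variant of the Revenant that restores its health instead of staying depleted.
; Each tick it refills health to 100 unless flinched, and its ServerDeath event also just resets health to 100.
; The overhead HP bar is turned toward the local camera every tick, rising and scaling up with camera distance.
; BeginPlay clears the take-damage camera shake, and the DamageIndicatorTick event is left empty.
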(event `self.ReceiveBeginPlay`
  (`parent.ReceiveBeginPlay`)
  (set `self.PlayerTakeDamageCameraShake` null))

(event `self.DamageIndicatorTick`)

(event `self.ReceiveTick`
  (params (DeltaSeconds :type "Float (single-precision)"))
  (bind _returnvalue (`GameplayStatics.GetPlayerCameraManager` 0))
  (bind _hpoverheadbp (`self.HPOverheadBP`))
  (bind (_relativelocation_x _relativelocation_y) (`KismetMathLibrary.BreakVector` (`SceneComponent.RelativeLocation` _hpoverheadbp)))
  (bind _returnvalue_2 (`KismetMathLibrary.VSize` (- (`SceneComponent.K2_GetComponentLocation` _hpoverheadbp) (`PlayerCameraManager.GetCameraLocation` _returnvalue))))
  (if (not (`self.Flinched`))
    (set `self.Health` 100.0))
  (`SceneComponent.K2_SetRelativeLocation` _hpoverheadbp (`KismetMathLibrary.MakeVector` _relativelocation_x _relativelocation_y (+ 100.0 (/ _returnvalue_2 20.0))) false false)
  (`SceneComponent.K2_SetWorldRotation` _hpoverheadbp (`KismetMathLibrary.MakeRotator` (.roll (`PlayerCameraManager.GetCameraRotation` _returnvalue)) (* (.pitch (`PlayerCameraManager.GetCameraRotation` _returnvalue)) -1.0) (+ (.yaw (`PlayerCameraManager.GetCameraRotation` _returnvalue)) 180.0)) false false)
  (`SceneComponent.SetRelativeScale3D` _hpoverheadbp (* (1.0 0.1 0.007) (+ 0.2 (/ _returnvalue_2 500.0)))))

(event `self.ServerDeath`
  (params (Attacker :type "BaseCharacter Object Reference"))
  (set `self.Health` 100.0))

(fn `UserConstructionScript`
  (`parent.UserConstructionScript`))