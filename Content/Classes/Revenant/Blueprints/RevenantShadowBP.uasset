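; Short-lived Revenant shadow actor that plays a random montage and then removes itself.
; After a brief delay on BeginPlay, it clears its blocking state and plays a montage picked at random from AnimArray, then destroys itself once a fixed delay ends.
; The construction script attaches the Shield component to the mesh's shield socket.
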(event `self.ReceiveBeginPlay`
  (bind _animarray (`self.AnimArray`))
  (`KismetSystemLibrary.Delay` 0.3)
  (set `self.IsBlocking` false)
  (set `self.BlockingAnim` 0.0)
  (`AnimInstance.Montage_Play` (`SkeletalMeshComponent.GetAnimInstance` (`self.Mesh`)) (`|GetArrayItem` _animarray (`KismetMathLibrary.RandomIntegerInRange` 0 (- (`KismetArrayLibrary.Array_Length` _animarray) 1))) 1.0 "MontageLength" 0.0)
  (`KismetSystemLibrary.Delay` 1.7)
  (`self.K2_DestroyActor`))

(fn `UserConstructionScript`
  (`SceneComponent.K2_AttachToComponent` (`self.Shield`) (`self.Mesh`) "Shieldsocket" "KeepRelative" "KeepRelative" "KeepRelative" true))