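; Base projectile for the Revenant class that destroys itself on hitting anything but its instigator and, on overlap, applies the effect picked by projectile name, here Impede.
; At close range, a target blocking toward the launch point plays a shield recoil; otherwise it flinches and takes damage, extending the attacker's active combo.
; Beyond that range, Impede skips the block check, slowing the target as well as damaging it.
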(event `self.ReceiveHit`
  (params (MyComp :type "PrimitiveComponent Object Reference") (Other :type "Actor Object Reference") (OtherComp :type "PrimitiveComponent Object Reference") (bSelfMoved :type Boolean) (HitLocation :type "Vector Structure") (HitNormal :type "Vector Structure") (NormalImpulse :type "Vector Structure") (Hit :type "HitResult Structure (by ref)"))
  (if (!= Other (`self.Instigator`))
    (`self.K2_DestroyActor`)))

(event `self.ReceiveActorBeginOverlap`
  (params (OtherActor :type "Actor Object Reference"))
  (bind _attacked (`self.Attacked`))
  (bind _attacker (`self.Attacker`))
  (if (!= OtherActor (`self.Instigator`))
    (set `self.Attacker` (cast `BaseCharacter` (`self.Instigator`) :!pure true))
    (set `self.Attacked` (cast `BaseCharacter` OtherActor :!pure true))
    (switch `string` (`self.ProjectileName`)
      (:`Impede`
        (if (< (`self.GetDistanceTo` (`self.Attacker`) (`self.Attacked`)) 400.0)
          (bind _blocked (`self.GetPlayerDirections` (`self.Attacked`)))
          (if (and _blocked (`BaseCharacter.IsBlocking` (`self.Attacked`)))
            (`BaseCharacter.PlayActionAnimServer` (`self.Attacked`) "/Game/Classes/Revenant/Animations/Recoil/Shield_Block_Recoil_Montage.Shield_Block_Recoil_Montage" 1.0)
            (else
              (if (> (`BaseCharacter.AttackCastCooldown` (`self.Attacker`)) (`KismetSystemLibrary.GetGameTimeInSeconds`))
                (set `BaseCharacter.LastAttack` "ComboExtender" (`self.Attacker`))
                (set `BaseCharacter.CurrentAttackHit` true (`self.Attacker`)))
              (set `BaseCharacter.FlinchTrigger` true (`self.Attacked`) :!label _label)
              (bind _returnvalue (`BaseCharacter.GetDamage` _attacker "Impede"))
              (`BaseCharacter.ApplyDamage` (`self.Attacked`) _returnvalue _attacker)))
          (else
            (set `BaseCharacter.FlinchTrigger` true _attacked)
            (`BaseCharacter.AddSpeedModifier` _attacked (* 230.0 -0.75) 3.0)
            (goto _label)))
        (`self.K2_DestroyActor`)))))

(fn `GetPlayerDirections`
  (params (Attacked :type "Actor Object Reference"))
  (returns (Blocked :type Boolean))
  (return (<= (`KismetMathLibrary.VSize` (- (`KismetMathLibrary.Conv_RotatorToVector` (`KismetMathLibrary.FindLookAtRotation` (`self.K2_GetActorLocation` Attacked) (`self.ProjectileStartLoc`))) (`KismetMathLibrary.GetForwardVector` (`self.K2_GetActorRotation` Attacked)))) 0.9)))

(fn `UserConstructionScript`)