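; Third-person locomotion character Blueprint handling camera-relative movement, landing, turn-in-place and physics ragdoll.
; Tick derives floor-relative velocity, sets walk speed, and either pushes down steep slopes or snaps the capsule to the ragdolled hips.
; Timelines drive camera changes, landing braking, turn rotation and ragdoll blending, with get-up montages chosen by hip roll.
; Jump, walk/sprint toggle and ragdoll trigger logic exists but is unconnected.
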(event `self.ReceiveBeginPlay`
  (`self.UpdateCameraSettings`))

(event `self.OnLanded`
  (params (Hit :type "HitResult Structure (by ref)"))
  (bind _charactermovement (`self.CharacterMovement`))
  (bind _returnvalue (`SkeletalMeshComponent.GetAnimInstance` (`self.Mesh`)))
  ;[1 1 1] CustomJump/LandingEvent
  (set `self.Jumped` false)
  (`|ExecutionSequence`
    (:`then_0`
      (bind (_direction _multiplier) (`Timeline|RampUpDecelerationOnLand` :!via `PlayFromStart`)
        (:`Update`
          (set `CharacterMovementComponent.BrakingDecelerationWalking` (* (`self.BrakingDeceleration`) _multiplier) _charactermovement))
        (:`Finished`
          (set `CharacterMovementComponent.BrakingDecelerationWalking` (`self.BrakingDeceleration`) _charactermovement))))
    (:`then_1`
      (if (not (or (`AnimInstance.Montage_IsPlaying` _returnvalue "/Game/Classes/Revenant/Animations/GettingUp/GetUpFromBack_Montage.GetUpFromBack_Montage") (`AnimInstance.Montage_IsPlaying` _returnvalue "/Game/Classes/Revenant/Animations/GettingUp/GetUpFromFront_Montage.GetUpFromFront_Montage")))
        (`self.PlayAnimMontage` "/Game/Classes/Revenant/Animations/InAir/LandingAdditive_Montage.LandingAdditive_Montage")))))

(event `self.ReceiveTick`
  (params (DeltaSeconds :type "Float (single-precision)"))
  (bind _capsulecomponent (`self.CapsuleComponent`))
  (bind _returnvalue (`SceneComponent.GetUpVector` _capsulecomponent))
  (bind _returnvalue_2 (`CapsuleComponent.GetScaledCapsuleRadius` _capsulecomponent))
  (bind (_bblockinghit _binitialoverlap _time _location _impactpoint _normal _impactnormal _physmat _hitactor _hitcomponent) (`GameplayStatics.BreakHitResult` (`.HitResult` (break `FindFloorResult` (`CharacterMovementComponent.CurrentFloor` (`self.CharacterMovement`))))))
  (bind _returnvalue_3 (`KismetSystemLibrary.IsValid` _hitcomponent))
  (bind _returnvalue_4 (+ (`.ImpactPoint` (`GameplayStatics.BreakHitResult` (`.HitResult` (break `FindFloorResult` (`CharacterMovementComponent.CurrentFloor` (`self.CharacterMovement`)))))) (* _returnvalue _returnvalue_2)))
  ;[1 1 1] EventTick
  (set `self.DeltaSeconds` DeltaSeconds)
  (`|ExecutionSequence`
    (:`then_0`
      (`|ExecutionSequence`
        (:`then_0`
          (bind _returnvalue_5 (`PrimitiveComponent.GetPhysicsLinearVelocity` (`self.CapsuleComponent`) "None"))
          (if _returnvalue_3
            (bind _returnvalue_6 (`PrimitiveComponent.GetPhysicsLinearVelocityAtPoint` _hitcomponent _impactpoint "None")))
          (if (`NavMovementComponent.IsFalling` (`self.CharacterMovement`))
            (bind _returnvalue_7 (- _returnvalue_5 (`KismetMathLibrary.SelectVector` _returnvalue_6 (0.0 0.0 0.0) _returnvalue_3)))
            (set `self.LastInAirVelocityVector` _returnvalue_7))
          (bind _output_get (set `self.VelocityVector` _returnvalue_7))
          (bind _x (.x _output_get))
          (bind _y (.y _output_get))
          (bind _returnvalue_8 (`KismetMathLibrary.MakeVector` _x _y))
          (set `self.Speed` (`KismetMathLibrary.VSize` (`KismetMathLibrary.SelectVector` _returnvalue_8 (`KismetMathLibrary.MakeVector` _x _y (.z _output_get)) (`NavMovementComponent.IsFalling` (`self.CharacterMovement`)))))
          (bind _output_get_2 (set `self.Moving` (!= _returnvalue_8 (0.0 0.0 0.0))))
          (if _output_get_2
            (set `self.LastVelocityRotation` (`KismetMathLibrary.Conv_VectorToRotator` _returnvalue_8))))
        (:`then_1`
          (set `self.MovementInput` (!= (`KismetMathLibrary.MakeVector` (.x (`PawnMovementComponent.GetLastInputVector` (`self.CharacterMovement`))) (.y (`PawnMovementComponent.GetLastInputVector` (`self.CharacterMovement`)))) (0.0 0.0 0.0) :`ErrorTolerance` 0.01)))))
    (:`then_1`
      (if (`self.OnSlope`)
        (set `CharacterMovementComponent.MaxWalkSpeed` 375.0 (`self.CharacterMovement`))
        (else
          (bind _output_get_3 (set `CharacterMovementComponent.MaxWalkSpeed` (`KismetMathLibrary.FInterpTo` (stale _output_get_3) (`KismetMathLibrary.SelectFloat` (`self.SprintSpeed`) (`KismetMathLibrary.SelectFloat` 190.0 230.0 (`self.ShouldWalk`)) (`self.ShouldSprint`)) (`self.DeltaSeconds`) 5.0) (`self.CharacterMovement`))))))
    (:`then_2`
      (if (`self.InRagdoll`)
        (`self.K2_SetActorLocation` (+ (`SceneComponent.GetSocketLocation` (`self.Mesh`) (`self.HipsBone`)) (`KismetMathLibrary.MakeVector` 0.0 0.0 (`CapsuleComponent.GetScaledCapsuleHalfHeight` (`self.CapsuleComponent`)))))
        (elif (not (`NavMovementComponent.IsFalling` (`self.CharacterMovement`)))
          (bind _outhit (`KismetSystemLibrary.SphereTraceSingle` _returnvalue_4 (+ _returnvalue_4 (* _returnvalue (* (+ _returnvalue_2 5.0) -1.0))) 1.0 "TraceTypeQuery1"))
          (bind (_bblockinghit_2 _binitialoverlap_2 _time_2 _location_2 _impactpoint_2 _normal_2) (`GameplayStatics.BreakHitResult` _outhit))
          (bind _z (.z _normal_2))
          (if (and _bblockinghit_2 (< _z 0.7) (> _z 0.1))
            (set `self.OnSlope` true)
            (`self.AddMovementInput` _normal_2)
            (`/Engine/EditorBlueprintResources/StandardMacros.DoOnce` false :!label _label
              (:`Completed`
                (bind (_direction _inputaxismultiplier) (`Timeline|SetMovementInputAxisMultiplier` :!via `PlayFromStart`)
                  (:`Update`
                    (set `self.MovementInputAxisMultiplier` _inputaxismultiplier)
                    (goto _label_2 :!via `Reset`)))))
            (else
              (set `self.OnSlope` false)
              (`/Engine/EditorBlueprintResources/StandardMacros.DoOnce` false :!label _label_2
                (:`Completed`
                  (set `self.MovementInputAxisMultiplier` 1.0)
                  (goto _label :!via `Reset`))))))))))

(event `TurnInPlace`
  (params (TurnInPlaceStart :type "Rotator Structure") (TurnInPlaceTarget :type "Rotator Structure") (Curve :type "CurveFloat Object Reference") (TurnAnimation :type "AnimMontage Object Reference"))
  (bind _turnlerpalpha (`self.TurnLerpAlpha`))
  ;[1 1 1] TurnInPlaceEvents
  (`/Engine/EditorBlueprintResources/StandardMacros.DoOnce` false :!label _label_3
    (:`Completed`
      (`|ExecutionSequence`
        (:`then_0`
          (set `self.TurningInPlace` true)
          (set `self.TurnInPlaceTarget` TurnInPlaceTarget)
          (set `self.TurnInPlaceStart` TurnInPlaceStart)
          (`TimelineComponent.SetFloatCurve` _turnlerpalpha Curve "Alpha")
          (`TimelineComponent.SetTimelineLength` _turnlerpalpha (`.MaxTime` (`CurveBase.GetTimeRange` Curve)))
          (`self.PlayAnimMontage` TurnAnimation)
          (bind (_direction _alpha) (`Timeline|TurnLerpAlpha` :!via `PlayFromStart` :!label _label_4)
            (:`Update`
              (set `self.TurnInPlaceRotation` (`KismetMathLibrary.RLerp` (`self.TurnInPlaceStart`) (`self.TurnInPlaceTarget`) _alpha)))
            (:`Finished`
              (`self.StopTurningInPlace`))))
        (:`then_1`
          (goto _label_5 :!via `Reset`))))))

(event `StopTurningInPlace`
  ;[1 1 1] TurnInPlaceEvents
  (`/Engine/EditorBlueprintResources/StandardMacros.DoOnce` false :!label _label_5
    (:`Completed`
      (`|ExecutionSequence`
        (:`then_0`
          (set `self.TurningInPlace` false)
          (`self.StopAnimMontage` (stale `TurnInPlace` TurnAnimation))
          (goto _label_4 :!via `Stop`))
        (:`then_1`
          (goto _label_3 :!via `Reset`))))))

(event `UnRagdoll`
  (bind _mesh (`self.Mesh`))
  (bind _mesh_2 (`self.Mesh`))
  (bind _capsulecomponent (`self.CapsuleComponent`))
  (bind _mesh_3 (`self.Mesh`))
  ;[1 1 1] RagdollBlending
  (if (`self.InRagdoll`)
    (set `self.InRagdoll` false)
    (`CharacterMovementComponent.SetMovementMode` (`self.CharacterMovement`) "MOVE_Falling" 0)
    (`PrimitiveComponent.SetCollisionObjectType` _mesh_3 "ECC_PhysicsBody")
    (`PrimitiveComponent.SetCollisionEnabled` _mesh_3 "QueryAndPhysics")
    (`PrimitiveComponent.SetCollisionObjectType` _capsulecomponent "ECC_Pawn")
    (`PrimitiveComponent.SetCollisionEnabled` _capsulecomponent "QueryOnly")
    (`self.UpdateCameraSettings`)
    (`|ExecutionSequence`
      (:`then_0`
        (`self.PlayAnimMontage` (select `bool` (> (.roll (`SceneComponent.GetSocketRotation` (`self.Mesh`) (`self.HipsBone`))) 0.0) :`false` "/Game/Classes/Revenant/Animations/GettingUp/GetUpFromBack_Montage.GetUpFromBack_Montage" :`true` "/Game/Classes/Revenant/Animations/GettingUp/GetUpFromFront_Montage.GetUpFromFront_Montage" :!type "AnimMontage Object Reference"))
        (bind (_direction _physicsblendweight) (`Timeline|UnRagdollBlend` :!via `PlayFromStart` :!label _label_6)
          (:`Update`
            (`SkeletalMeshComponent.SetAllBodiesBelowPhysicsBlendWeight` _mesh (`self.HipsBone`) _physicsblendweight false true))
          (:`Finished`
            (`PrimitiveComponent.SetSimulatePhysics` _mesh false))))
      (:`then_1`
        (bind (_direction_2 _spring) (`Timeline|RagdollBlend` :!via `Stop` :!label _label_7)
          (:`Update`
            (`SkeletalMeshComponent.SetAllMotorsAngularDriveParams` _mesh_2 _spring 0.0 100000.0 true))
          (:`Finished`
            (set `SkeletalMeshComponent.bUpdateJointsFromAnimation` false _mesh_2)
            (`SkeletalMeshComponent.SetAllMotorsAngularDriveParams` _mesh_2 0.0 0.0 0.0 false)))))))

(event `ToRagdoll`
  (bind _mesh (`self.Mesh`))
  (bind _capsulecomponent (`self.CapsuleComponent`))
  (bind _mesh_2 (`self.Mesh`))
  ;[1 1 1] RagdollBlending
  (if (not (`self.InRagdoll`))
    (set `self.InRagdoll` true)
    (`CharacterMovementComponent.SetMovementMode` (`self.CharacterMovement`) "MOVE_None" 0)
    (`PrimitiveComponent.SetCollisionObjectType` _mesh_2 "ECC_PhysicsBody")
    (`PrimitiveComponent.SetCollisionEnabled` _mesh_2 "QueryAndPhysics")
    (`PrimitiveComponent.SetCollisionObjectType` _capsulecomponent "ECC_Pawn")
    (`PrimitiveComponent.SetCollisionEnabled` _capsulecomponent "QueryOnly")
    (`self.UpdateCameraSettings`)
    (`|ExecutionSequence`
      (:`then_0`
        (`SkeletalMeshComponent.SetAllBodiesBelowSimulatePhysics` _mesh (`self.HipsBone`) true true)
        (set `SkeletalMeshComponent.bUpdateJointsFromAnimation` false _mesh)
        (goto _label_7 :!via `PlayFromStart`))
      (:`then_1`
        (goto _label_6 :!via `Stop`)))))

(event `InputAxis|MoveForward`
  (params (AxisValue :type "Float (single-precision)"))
  (bind _returnvalue (* AxisValue (`self.MovementInputAxisMultiplier`)))
  (bind _returnvalue_2 (`KismetMathLibrary.MakeRotator` 0.0 0.0 (.yaw (`self.GetControlRotation`))))
  (bind _returnvalue_3 (`KismetMathLibrary.GetForwardVector` _returnvalue_2))
  ;[1 1 1] PlayerMovementInput
  (`|ExecutionSequence`
    (:`then_0`
      (set `self.PlayerMovementInputVector` (+ (* _returnvalue_3 _returnvalue) (* (`KismetMathLibrary.GetRightVector` _returnvalue_2) (* (stale `InputAxis|MoveRight` AxisValue) (`self.MovementInputAxisMultiplier`)))) :!label _label_8))
    (:`then_1`
      (if (`self.CanMove`)
        (`self.AddMovementInput` _returnvalue_3 _returnvalue)))))

(event `UpdateCameraSettings`
  (bind _tpspringarm (`self.TPSpringArm`))
  ;[1 1 1] UpdateCamera
  (`|ExecutionSequence`
    (:`then_0`
      (set `self.CurrentTargetArmLength` (`SpringArmComponent.TargetArmLength` _tpspringarm))
      (set `self.CurrentCameraLagSpeed` (`SpringArmComponent.CameraLagSpeed` _tpspringarm))
      (set `self.CurrentCameraSocketOffset` (`SpringArmComponent.SocketOffset` _tpspringarm))
      (bind (_direction _alpha) (`Timeline|CameraUpdate` :!via `PlayFromStart`)
        (:`Update`
          (if (`self.InRagdoll`)
            (set `SpringArmComponent.TargetArmLength` (`KismetMathLibrary.Lerp` (`self.CurrentTargetArmLength`) 210.0 _alpha) (`self.TPSpringArm`))
            (set `SpringArmComponent.CameraLagSpeed` (`KismetMathLibrary.Lerp` 3.0 3.0 _alpha) (`self.TPSpringArm`))
            (set `SpringArmComponent.SocketOffset` (`KismetMathLibrary.VLerp` (`self.CurrentCameraSocketOffset`) (0.0 0.0 -90.0) _alpha) (`self.TPSpringArm`))
            (else
              (set `SpringArmComponent.TargetArmLength` (`KismetMathLibrary.Lerp` (`self.CurrentTargetArmLength`) 160.0 _alpha) (`self.TPSpringArm`))
              (set `SpringArmComponent.CameraLagSpeed` (`KismetMathLibrary.Lerp` (`self.CurrentCameraLagSpeed`) 0.0 _alpha) (`self.TPSpringArm`))
              (set `SpringArmComponent.SocketOffset` (`KismetMathLibrary.VLerp` (`self.CurrentCameraSocketOffset`) (0.0 40.0 25.0) _alpha) (`self.TPSpringArm`)))))))
    (:`then_1`
      (`ActorComponent.SetActive` (`self.TPCamera`) true false)
      (`ActorComponent.SetActive` (`self.FPCamera`) false false))))

(event `InputAxis|MoveRight`
  (params (AxisValue :type "Float (single-precision)"))
  ;[1 1 1] PlayerMovementInput
  (`|ExecutionSequence`
    (:`then_0`
      (goto _label_8))
    (:`then_1`
      (if (`self.CanMove`)
        (`self.AddMovementInput` (`KismetMathLibrary.GetRightVector` (`KismetMathLibrary.MakeRotator` 0.0 0.0 (.yaw (`self.GetControlRotation`)))) (* AxisValue (`self.MovementInputAxisMultiplier`)))))))

(event `InputAxis|LookUp`
  (params (AxisValue :type "Float (single-precision)"))
  ;[1 1 1] CameraInput
  (if (`self.CanTurn`)
    (`self.AddControllerPitchInput` (* (* 150.0 AxisValue) (`self.DeltaSeconds`)))))

(event `InputAxis|Turn`
  (params (AxisValue :type "Float (single-precision)"))
  ;[1 1 1] CameraInput
  (if (`self.CanTurn`)
    (`self.AddControllerYawInput` (* (* AxisValue 150.0) (`self.DeltaSeconds`)))))

(fn `UserConstructionScript`)