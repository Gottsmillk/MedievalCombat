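; AI-controlled Revenant character Blueprint that serves as a thin host for an Advanced Locomotion System (ALS V2) component.
; It forwards movement mode changes, custom movement updates and landing events to that component.
; Tick calls a function meant to send movement input vectors for the AnimBP, but that function's body is empty.
; The movement mode getter graphs contain only unconnected nodes.
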(event `self.ReceiveBeginPlay`)

(event `self.ReceiveTick`
  (params (DeltaSeconds :type "Float (single-precision)"))
  ;[1 1 1] Tick Events
)

(event `self.K2_OnMovementModeChanged`
  (params (PrevMovementMode :type "EMovementMode Enum" :default "MOVE_None") (NewMovementMode :type "EMovementMode Enum" :default "MOVE_None") (PrevCustomMode :type Byte) (NewCustomMode :type Byte))
  ;[1 1 1] Character Events needed in ALS_Component
  (`/Game/Classes/RevenantOld/Blueprints/RevenantOld_Component.OnMovementModeChangeEvent` (`self.ALS_Component`) PrevMovementMode NewMovementMode PrevCustomMode NewCustomMode))

(event `self.K2_UpdateCustomMovement`
  (params (DeltaTime :type "Float (single-precision)"))
  ;[1 1 1] Character Events needed in ALS_Component
  (`/Game/Classes/RevenantOld/Blueprints/RevenantOld_Component.UpdateCustomMovementModeEvent` (`self.ALS_Component`)))

(event `self.OnLanded`
  (params (Hit :type "HitResult Structure (by ref)"))
  ;[1 1 1] Character Events needed in ALS_Component
  (`/Game/Classes/RevenantOld/Blueprints/RevenantOld_Component.LandEvent` (`self.ALS_Component`)))

(fn `UserConstructionScript`)