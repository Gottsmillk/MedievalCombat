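; RevenantOld movement component for a networked character, handling input, jumping, landing braking, locomotion states and walk/run/sprint speeds.
; Changes apply locally, then pass through server events to non-local copies.
; Ragdoll is a custom movement mode steered by pelvis torque; the controlling client moves the actor to the pelvis with ground-trace correction, while other copies force the pelvis toward the shared location.
; Leaving ragdoll restores velocity, snapshots the pose and plays a get-up montage.
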(event `OnMovementModeChangeEvent`
  (params (PrevMovementMode :type "EMovementMode Enum") (NewMovmentMode :type "EMovementMode Enum") (PrevCustomMovementMode :type Byte) (NewCustomMovementMode :type Byte))
  ;[1 1 1] Tick Events
  (`self.OnMovementModeChange` PrevMovementMode NewMovmentMode PrevCustomMovementMode NewCustomMovementMode)
  (`self.UpdateCamera`))

(event `SwitchMovementModeEvent`
  (params (MovementMode :type "EMovementMode Enum") (CustomMovementMode :type "/Game/Classes/RevenantOld/Blueprints/Enums/CustomMovementModes Enum"))
  ;[1 1 1] Tick Events
  (`CharacterMovementComponent.SetMovementMode` (`self.CharacterMovement`) MovementMode CustomMovementMode)
  (`self.SwitchMovementModeOnServer` MovementMode CustomMovementMode))

(event `SwitchMovementModeOnServer`
  (params (NewMovementMode :type "EMovementMode Enum") (NewCustomMode :type Byte))
  ;[1 1 1] Tick Events
  (`self.HasAuthority`
    (:`Authority`
      (`self.SwitchMovementModeOnAll` NewMovementMode NewCustomMode))))

(event `SwitchMovementModeOnAll`
  (params (NewMovementMode :type "EMovementMode Enum") (NewCustomMode :type Byte))
  ;[1 1 1] Tick Events
  (`self.IsLocallyControlled`
    (:`false`
      (`CharacterMovementComponent.SetMovementMode` (`self.CharacterMovement`) NewMovementMode NewCustomMode))))

(event `UpdateRagdollOnServer`
  (params (`Ragdoll Velocity` :type "Vector Structure") (RagdollLocation :type "Vector Structure") (ActorLocation :type "Vector Structure"))
  ;[1 1 1] Tick Events
  (`self.HasAuthority`
    (:`Authority`
      (`self.UpdateRagdollOnAll` `Ragdoll Velocity` RagdollLocation ActorLocation))))

(event `UpdateRagdollOnAll`
  (params (`Ragdoll Velocity` :type "Vector Structure") (RagdollLocation :type "Vector Structure") (ActorLocation :type "Vector Structure"))
  ;[1 1 1] Tick Events
  (`self.IsLocallyControlled`
    (:`false`
      (set `self.RagdollVelocity` `Ragdoll Velocity`)
      (set `self.RagdollLocation` RagdollLocation)
      (`Actor.K2_SetActorLocation` (`self.Pawn`) ActorLocation false false))))

(event `UpdateCustomMovementModeEvent`
  (bind _pelvisbone (`self.PelvisBone`))
  (bind _mesh (`self.Mesh`))
  (bind _returnvalue (`SceneComponent.GetSocketLocation` _mesh _pelvisbone))
  ;[1 1 1] Tick Events
  (switch `/Game/Classes/RevenantOld/Blueprints/Enums/CustomMovementModes` (`self.GetCustomMovementMode`)
    (:`NewEnumerator0`
      (`self.IsLocallyControlled`
        (:`true`
          (bind _returnvalue_2 (`PrimitiveComponent.GetPhysicsLinearVelocity` _mesh _pelvisbone))
          (bind _output_get (set `self.RagdollVelocity` _returnvalue_2))
          (bind _output_get_2 (set `self.RagdollLocation` _returnvalue))
          (bind _actorlocation (`self.CalculateActorLocationInRagdoll` _returnvalue))
          (`Actor.K2_SetActorLocation` (`self.Pawn`) _actorlocation false false)
          (`self.UpdateRagdollOnServer` _output_get _output_get_2 _actorlocation))))))

(event `ToRagdoll`
  (bind _mesh (`self.Mesh`))
  ;[1 1 1] Tick Events
  (`Character.SetReplicateMovement` (`self.Character`) false)
  (`PrimitiveComponent.SetCollisionEnabled` (`self.CapsuleComponent`) "NoCollision")
  (`PrimitiveComponent.SetCollisionObjectType` _mesh "ECC_PhysicsBody")
  (`PrimitiveComponent.SetCollisionEnabled` _mesh "QueryAndPhysics")
  (`SkeletalMeshComponent.SetAllBodiesBelowSimulatePhysics` (`self.Mesh`) (`self.PelvisBone`) true true)
  (set `SkeletalMeshComponent.bUpdateJointsFromAnimation` true (`self.Mesh`)))

(event `UnRagdoll`
  (bind _mesh (`self.Mesh`))
  ;[1 1 1] Tick Events
  (set `MovementComponent.Velocity` (`self.RagdollVelocity`) (`self.CharacterMovement`))
  (`AnimInstance.SavePoseSnapshot` (`self.AnimInstance`) "RagdollPose")
  (`Character.SetReplicateMovement` (`self.Character`) true)
  (`PrimitiveComponent.SetCollisionEnabled` (`self.CapsuleComponent`) "QueryAndPhysics")
  (`AnimInstance.Montage_Play` (`self.AnimInstance`) (`self.ChooseGetUpMontage`) 1.5 "MontageLength" 0.0)
  (`PrimitiveComponent.SetCollisionObjectType` _mesh "ECC_Pawn")
  (`PrimitiveComponent.SetCollisionEnabled` _mesh "QueryOnly")
  (`SkeletalMeshComponent.SetAllBodiesSimulatePhysics` _mesh false))

(event `self.ReceiveBeginPlay`
  ;[1 1 1] Initialize Component
  (`self.SetReferences`)
  (`self.SetDefaultSettings`))

(event `self.ReceiveTick`
  (params (DeltaSeconds :type "Float (single-precision)"))
  (bind _returnvalue (`SceneComponent.GetSocketLocation` (`self.Mesh`) (`self.PelvisBone`)))
  ;[1 1 1] Tick Events
  (switch `EMovementMode` (`self.GetMovementMode`)
    (:`MOVE_Custom`
      (switch `/Game/Classes/RevenantOld/Blueprints/Enums/CustomMovementModes` (`self.GetCustomMovementMode`)
        (:`NewEnumerator0`
          (bind _returnvalue_2 (`PrimitiveComponent.GetPhysicsLinearVelocity` (`self.Mesh`) (`self.PelvisBone`)))
          (`SkeletalMeshComponent.SetAllMotorsAngularDriveParams` (`self.Mesh`) (`KismetMathLibrary.MapRangeClamped` (`KismetMathLibrary.VSize` _returnvalue_2) 0.0 1000.0 0.0 25000.0) 0.0 0.0 false)
          (`self.IsLocallyControlled`
            (:`false`
              (`PrimitiveComponent.AddForceAtLocation` (`self.Mesh`) (* (- (`self.RagdollLocation`) _returnvalue) 200.0) _returnvalue (`self.PelvisBone`)))))))))

(event `PlayerMovementInputEvent`
  (params (ForwardAxis :type "Float (double-precision)") (RightAxis :type "Float (double-precision)"))
  (bind (_forwardvector _rightvector) (`self.GetForward/RightVector`))
  (bind (_forwardvector_2 _rightvector_2) (`self.GetForward/RightVector`))
  (bind _pawn (`self.Pawn`))
  (bind (_returnvalue_x _returnvalue_y _returnvalue_z) (`KismetMathLibrary.BreakVector` (* (`KismetMathLibrary.Normal` (+ (* _forwardvector_2 (`self.MoveForward/BackwardsAxisValue`)) (* _rightvector_2 (`self.MoveRight/LeftAxisValue`)))) (`KismetMathLibrary.SelectFloat` 500.0 250.0 (`self.Sprinting`)))))
  ;[1 1 1] Player Movement Input Event
  (`self.SetPlayerMovementAxisValues` ForwardAxis RightAxis)
  (switch `EMovementMode` (`self.GetMovementMode`)
    (:`MOVE_Walking`
      (`Pawn.AddMovementInput` _pawn _forwardvector (`self.MoveForward/BackwardsAxisValue`) false :!label _label)
      (`Pawn.AddMovementInput` _pawn _rightvector (`self.MoveRight/LeftAxisValue`) false))
    (:`MOVE_NavWalking`
      (goto _label))
    (:`MOVE_Falling`
      (goto _label))
    (:`MOVE_Flying`
      (goto _label))
    (:`MOVE_Custom`
      (switch `/Game/Classes/RevenantOld/Blueprints/Enums/CustomMovementModes` (`self.GetCustomMovementMode`)
        (:`NewEnumerator0`
          (`self.IsLocallyControlled`
            (:`true`
              (`PrimitiveComponent.AddTorque` (`self.Mesh`) (`KismetMathLibrary.MakeVector` (* _returnvalue_y -1.0) _returnvalue_x _returnvalue_z) (`self.PelvisBone`) true))))))))

(event `SetMovementInputVectorOnServer`
  (params (MovmentInputVector :type "Vector Structure"))
  ;[1 1 1] Set Movement Input Vector
  (`self.HasAuthority`
    (:`Authority`
      (`self.SetMovementInputVectorOnAll` MovmentInputVector))))

(event `SetMovementInputVectorOnAll`
  (params (MovementInputVector :type "Vector Structure"))
  ;[1 1 1] Set Movement Input Vector
  (`self.IsLocallyControlled`
    (:`false`
      (set `self.MovementInputVector` MovementInputVector))))

(event `SetMovementInputVectorEvent`
  (params (MovementInputVector :type "Vector Structure"))
  ;[1 1 1] Set Movement Input Vector
  (bind _output_get (set `self.MovementInputVector` MovementInputVector))
  (`self.SetMovementInputVectorOnServer` _output_get))

(event `UpdateMovementSpeedEvent`
  (params (Sprinting :type Boolean) (Walking :type Boolean))
  ;[1 1 1] Update Movement Settings/Speed
  (bind _output_get (set `self.Sprinting` Sprinting))
  (bind _output_get_2 (set `self.Walking` Walking))
  (bind _output_get_3 (set `CharacterMovementComponent.MaxWalkSpeed` (`self.ChooseMaxWalkSpeed`) (`self.CharacterMovement`)))
  (`self.UpdateMovementSpeedOnServer` _output_get_3 _output_get _output_get_2)
  (`self.UpdateCamera`))

(event `UpdateMovementSpeedOnServer`
  (params (MaxWalkSpeed :type "Float (double-precision)") (Sprinting :type Boolean) (Walking :type Boolean))
  ;[1 1 1] Update Movement Settings/Speed
  (`self.HasAuthority`
    (:`Authority`
      (`self.UpdateMovementSpeedOnAll` MaxWalkSpeed Sprinting Walking))))

(event `UpdateMovementSpeedOnAll`
  (params (MaxWalkSpeed :type "Float (double-precision)") (Sprinting :type Boolean) (Walking :type Boolean))
  ;[1 1 1] Update Movement Settings/Speed
  (`self.IsLocallyControlled`
    (:`false`
      (set `CharacterMovementComponent.MaxWalkSpeed` MaxWalkSpeed (`self.CharacterMovement`))
      (set `self.Sprinting` Sprinting)
      (set `self.Walking` Walking))))

(event `UpdateMovementSettingsEvent`
  (params (MaxAcceleration :type "Float (double-precision)") (BrakingDecelerationWalking :type "Float (double-precision)") (GroundFriction :type "Float (double-precision)") (JumpZVelocity :type "Float (double-precision)"))
  (bind _charactermovement (`self.CharacterMovement`))
  ;[1 1 1] Update Movement Settings/Speed
  (bind _output_get (set `CharacterMovementComponent.MaxAcceleration` MaxAcceleration _charactermovement))
  (bind _output_get_2 (set `CharacterMovementComponent.BrakingDecelerationWalking` BrakingDecelerationWalking _charactermovement))
  (bind _output_get_3 (set `CharacterMovementComponent.GroundFriction` GroundFriction _charactermovement))
  (bind _output_get_4 (set `CharacterMovementComponent.JumpZVelocity` JumpZVelocity _charactermovement))
  (`self.UpdateMovementSettingsOnServer` _output_get _output_get_2 _output_get_3 _output_get_4))

(event `UpdateMovementSettingsOnServer`
  (params (MaxAcceleration :type "Float (double-precision)") (BrakingDecelerationWalking :type "Float (double-precision)") (GroundFriction :type "Float (double-precision)") (JumpZVelocity :type "Float (double-precision)"))
  ;[1 1 1] Update Movement Settings/Speed
  (`self.HasAuthority`
    (:`Authority`
      (`self.UpdateMovementSettingsOnAll` MaxAcceleration BrakingDecelerationWalking GroundFriction JumpZVelocity))))

(event `UpdateMovementSettingsOnAll`
  (params (MaxAcceleration :type "Float (double-precision)") (BrakingDecelerationWalking :type "Float (double-precision)") (GroundFriction :type "Float (double-precision)") (JumpZVelocity :type "Float (double-precision)"))
  (bind _charactermovement (`self.CharacterMovement`))
  ;[1 1 1] Update Movement Settings/Speed
  (`self.IsLocallyControlled`
    (:`false`
      (set `CharacterMovementComponent.MaxAcceleration` MaxAcceleration _charactermovement)
      (set `CharacterMovementComponent.BrakingDecelerationWalking` BrakingDecelerationWalking _charactermovement)
      (set `CharacterMovementComponent.GroundFriction` GroundFriction _charactermovement)
      (set `CharacterMovementComponent.JumpZVelocity` JumpZVelocity _charactermovement))))

(event `SwitchLocomotionStateEvent`
  (params (LocomotionState :type "/Game/Classes/RevenantOld/Blueprints/Enums/LocomotionState Enum"))
  ;[1 1 1] Switch Locomotion State
  (bind _output_get (set `self.LocomotionState` LocomotionState))
  (`self.SwitchLocomotionStateOnServer` _output_get)
  (`self.UpdateMovementSpeedEvent` (`self.Sprinting`) (`self.Walking`)))

(event `SwitchLocomotionStateOnServer`
  (params (LocomotionState :type "/Game/Classes/RevenantOld/Blueprints/Enums/LocomotionState Enum"))
  ;[1 1 1] Switch Locomotion State
  (`self.HasAuthority`
    (:`Authority`
      (`self.SwitchLocomotionStateOnAll` LocomotionState))))

(event `SwitchLocomotionStateOnAll`
  (params (LocomotionState :type "/Game/Classes/RevenantOld/Blueprints/Enums/LocomotionState Enum"))
  ;[1 1 1] Switch Locomotion State
  (`self.IsLocallyControlled`
    (:`false`
      (set `self.LocomotionState` LocomotionState))))

(event `JumpEvent`
  ;[1 1 1] Jump/Landing
  (`Character.Jump` (`self.Character`)))

(event `LandEvent`
  ;[1 1 1] Jump/Landing
  (set `CharacterMovementComponent.BrakingDecelerationWalking` (+ (`self.BrakingDeceleration`) 2000.0) (`self.CharacterMovement`))
  (`KismetSystemLibrary.RetriggerableDelay` 0.2)
  (set `CharacterMovementComponent.BrakingDecelerationWalking` (`self.BrakingDeceleration`) (`self.CharacterMovement`)))

(fn `CalculateActorLocationInRagdoll`
  (params (RagdollLocation :type "Vector Structure"))
  (returns (ActorLocation :type "Vector Structure"))
  (bind _outhit (`KismetSystemLibrary.LineTraceSingle` RagdollLocation (- RagdollLocation (0.0 0.0 50.0)) "TraceTypeQuery1"))
  (bind (_bblockinghit _binitialoverlap _time _location) (`GameplayStatics.BreakHitResult` _outhit))
  (bind (_returnvalue_x _returnvalue_y _returnvalue_z) (`KismetMathLibrary.BreakVector` (- RagdollLocation _location)))
  (bind _returnvalue (`KismetMathLibrary.FInterpTo` (stale _output_get) (`KismetMathLibrary.SelectFloat` _returnvalue_z 0.0 _bblockinghit) (`GameplayStatics.GetWorldDeltaSeconds`) 5.0))
  (bind _output_get (set `self.ZOffset` _returnvalue))
  (return (+ RagdollLocation (`KismetMathLibrary.MakeVector` 0.0 0.0 (- (`CapsuleComponent.GetScaledCapsuleHalfHeight` (`self.CapsuleComponent`)) _returnvalue)))))

(fn `OnMovementModeChange`
  (params (PrevMovementMode :type "EMovementMode Enum") (NewMovementMode :type "EMovementMode Enum") (PrevCustomMovementMode :type Byte) (NewCustomMovementMode :type Byte))
  (locals (`NewMovementMode ` :type "EMovementMode Enum") (`NewCustomMovementMode ` :type "/Game/Classes/RevenantOld/Blueprints/Enums/CustomMovementModes Enum"))
  (set `self.PrevMovementMode` PrevMovementMode)
  (set `local.NewMovementMode ` NewMovementMode)
  (set `self.PrevCustomMovementMode` (cast `/Game/Classes/RevenantOld/Blueprints/Enums/CustomMovementModes` PrevCustomMovementMode))
  (set `local.NewCustomMovementMode ` (cast `/Game/Classes/RevenantOld/Blueprints/Enums/CustomMovementModes` NewCustomMovementMode))
  (`|ExecutionSequence`
    (:`then_0`
      ;[1 1 1] Previous Movement Mode
      (switch `EMovementMode` (`self.PrevMovementMode`)
        (:`MOVE_Custom`
          (switch `/Game/Classes/RevenantOld/Blueprints/Enums/CustomMovementModes` (`self.PrevCustomMovementMode`)
            (:`NewEnumerator0`
              (`self.UnRagdoll`))))))
    (:`then_1`
      ;[1 1 1] New Movement Mode
      (switch `EMovementMode` (`local.NewMovementMode `)
        (:`MOVE_Custom`
          (switch `/Game/Classes/RevenantOld/Blueprints/Enums/CustomMovementModes` (`local.NewCustomMovementMode `)
            (:`NewEnumerator0`
              (`self.ToRagdoll`))))))))

(fn `SetDefaultSettings`
  (`self.UpdateMovementSettingsEvent` (`self.MaxAcceleration`) (`self.BrakingDeceleration`) (`self.GroundFriction`) (`self.JumpVelocity`))
  (`self.UpdateMovementSpeedEvent` (`self.Sprinting`) (`self.Walking`)))

(fn `SetPlayerMovementAxisValues`
  (params (ForwardAxis :type "Float (double-precision)") (RightAxis :type "Float (double-precision)"))
  (bind _movementinputaxismultiplier (`self.MovementInputAxisMultiplier`))
  (set `self.MoveForward/BackwardsAxisValue` (* ForwardAxis _movementinputaxismultiplier))
  (set `self.MoveRight/LeftAxisValue` (* RightAxis _movementinputaxismultiplier)))

(fn `SetReferences`
  (bind _returnvalue (`Actor.GetComponentByClass` (`self.Pawn`) "/Script/Engine.SkeletalMeshComponent"))
  (bind _returnvalue_2 (`Actor.GetComponentByClass` (`self.Pawn`) "/Script/Engine.CapsuleComponent"))
  ;[1 1 1] Set Reference To Pawn
  (bind _aspawn (cast `Pawn` (`self.GetOwner`)))
  (set `self.Pawn` _aspawn)
  (`|ExecutionSequence`
    (:`then_0`
      ;[1 1 1] Set Character Reference
      (bind _ascharacter (cast `Character` (`self.Pawn`)))
      (set `self.Character` _ascharacter))
    (:`then_1`
      ;[1 1 1] Set Character Movement Component Reference
      (bind _ascharacter_movement_component (cast `CharacterMovementComponent` (`Pawn.GetMovementComponent` (`self.Pawn`))))
      (set `self.CharacterMovement` _ascharacter_movement_component))
    (:`then_2`
      ;[1 1 1] Set Capsule Reference
      (`/Engine/EditorBlueprintResources/StandardMacros.IsValid` _returnvalue_2
        (:`Is Valid`
          (set `self.CapsuleComponent` _returnvalue_2))))
    (:`then_3`
      ;[1 1 1] Set Skeletal Mesh and Anim Instance Reference
      (`/Engine/EditorBlueprintResources/StandardMacros.IsValid` _returnvalue
        (:`Is Valid`
          (bind _output_get (set `self.Mesh` _returnvalue))
          (bind _returnvalue_3 (`SkeletalMeshComponent.GetAnimInstance` _output_get))
          (`/Engine/EditorBlueprintResources/StandardMacros.IsValid` _returnvalue_3
            (:`Is Valid`
              (set `self.AnimInstance` _returnvalue_3))))))))