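; Player controller for the training grounds that drives character selection and the menu widgets.
; On start it shows character select and a hidden in-game menu that Escape reveals.
; Choosing a character asks the TrainingGroundsGamemode to spawn the player, then opens the Revenant attack-selection menu, removing any existing HUD.
; A key rebinding screen lists every action binding from the Victory plugin as Rama-style widget rows.
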(event `self.ReceiveBeginPlay`
  (bind _returnvalue (`|CreateWidget` "/Game/Menus/IngameUI/IngameMenu.IngameMenu_C"))
  (bind _output_get (set `self.IngameMenu` _returnvalue))
  (`Widget.SetVisibility` _output_get "Hidden")
  (`UserWidget.AddToViewport` _output_get 0)
  (bind _returnvalue_2 (`|CreateWidget` "/Game/Menus/Lobby/CharacterSelect.CharacterSelect_C"))
  (bind _output_get_2 (set `self.Character Select` _returnvalue_2))
  (`UserWidget.AddToViewport` _output_get_2 0)
  (set `self.bShowMouseCursor` true))

(event `Key|Escape`
  (params (Key :type "Key Structure"))
  (bind _ingamemenu (`self.IngameMenu`))
  (:`Pressed`
    (`Widget.SetVisibility` _ingamemenu "Visible")
    (`WidgetBlueprintLibrary.SetInputMode_UIOnlyEx` self _ingamemenu)
    (set `self.bShowMouseCursor` true)))

(event `DisplayKeybinds`
  (bind _rebindmenu (`self.RebindMenu`))
  ;[1 1 1] Display Keybinds
  (bind _returnvalue (`|CreateWidget` "/Game/Menus/Rebind/Main_ByRama.Main_ByRama_C"))
  (bind _output_get (set `self.RebindMenu` _returnvalue))
  (`UserWidget.AddToViewport` _output_get 0)
  (`WidgetBlueprintLibrary.SetInputMode_UIOnlyEx` self (`self.RebindMenu`))
  (set `self.bShowMouseCursor` true)
  (for _array_element (`VictoryBPFunctionLibrary.VictoryGetAllActionKeyBindings`)
    (bind _returnvalue_2 (`|CreateWidget` "/Game/Menus/Rebind/Element_ByRama.Element_ByRama_C"))
    (set `/Game/Menus/Rebind/Element_ByRama.Main` _rebindmenu _returnvalue_2)
    (`PanelWidget.AddChild` (`/Game/Menus/Rebind/Main_ByRama.MainScroll` _rebindmenu) (`/Game/Menus/Rebind/Element_ByRama.Core` _returnvalue_2))
    (`/Game/Menus/Rebind/Element_ByRama.SetValues` _returnvalue_2 _array_element)))

(event `StartUI`
  (bind _returnvalue (`|CreateWidget` "/Game/Classes/Revenant/Blueprints/UI.UI_C"))
  (bind _output_get (set `self.IngameUI` _returnvalue))
  (`UserWidget.AddToViewport` _output_get 0))

(event `Open Choose Menu`
  (bind _ingameui (`self.IngameUI`))
  ;[1 1 1] Open Menu for choosing attacks
  (`/Engine/EditorBlueprintResources/StandardMacros.IsValid` _ingameui
    (:`Is Valid`
      (`Widget.RemoveFromParent` _ingameui))
    (:`Is Not Valid`
      _))
  (bind _returnvalue (`|CreateWidget` "/Game/Classes/Revenant/Blueprints/RevenantChooseAttacks.RevenantChooseAttacks_C"))
  (`UserWidget.AddToViewport` _returnvalue 0)
  (`WidgetBlueprintLibrary.SetInputMode_UIOnlyEx` self _returnvalue)
  (set `self.bShowMouseCursor` true))

(event `ChooseCharacter`
  (params (`Class ID` :type Integer))
  (`/Game/Blueprints/GameplayBPs/TrainingGroundsGamemode.SpawnPlayer` (cast `/Game/Blueprints/GameplayBPs/TrainingGroundsGamemode` (`GameplayStatics.GetGameMode`) :!pure true) `Class ID` self)
  (set `self.bShowMouseCursor` false)
  (`self.Open Choose Menu`))

(fn `UserConstructionScript`)