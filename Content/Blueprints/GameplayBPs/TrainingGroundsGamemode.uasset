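; Game mode for the training grounds that spawns players as a chosen character class.
; SpawnPlayer destroys the controller's current pawn if valid, then spawns the class indexed by ClassID in CharacterList at a random PlayerStart, adjusting for collisions but always spawning.
; The controller possesses the new pawn and switches to game-only input.
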(event `SpawnPlayer`
  (params (`Class ID` :type Integer) (Controller :type "PlayerController Object Reference"))
  (bind _returnvalue (`Controller.K2_GetPawn` Controller))
  (bind _spawn_points (`self.Spawn Points`))
  (bind _outactors (`GameplayStatics.GetAllActorsOfClass` "/Script/Engine.PlayerStart"))
  (set `self.Spawn Points` _outactors)
  (`/Engine/EditorBlueprintResources/StandardMacros.IsValid` _returnvalue
    (:`Is Valid`
      (`self.K2_DestroyActor` _returnvalue))
    (:`Is Not Valid`
      _))
  (bind _returnvalue_2 (`|SpawnActorFromClass` (`|GetArrayItem` (`self.CharacterList`) `Class ID`) (`self.GetTransform` (`|GetArrayItem` _spawn_points (`KismetMathLibrary.RandomIntegerInRange` 0 (- (`KismetArrayLibrary.Array_Length` _spawn_points) 1)))) "AdjustIfPossibleButAlwaysSpawn" "OverrideRootScale" null null))
  (`Controller.Possess` Controller _returnvalue_2)
  (`WidgetBlueprintLibrary.SetInputMode_GameOnly` Controller))

(fn `UserConstructionScript`)