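; Game state for duel matches that runs the round loop, scores, scoreboard visibility and match end.
; Looping timers drive a pre-round countdown that unlocks players, then a round clock that freezes them on expiry.
; OnScored awards living players a point; either round ending shows the scoreboard, then resets players for another round.
; Three points, or a two-player score comparison at MaxRounds, triggers GameOver, which displays the result, opens MainMenu and destroys the session.
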(event `SetPlayerData`
  (params (IngamePC :type "/Game/Blueprints/GameplayBPs/IngamePC Object Reference"))
  (`KismetArrayLibrary.Array_AddUnique` (`self.PlayerScoreArray`) (make `/Game/Blueprints/GameplayBPs/IngamePlayerScoreList` IngamePC 0 (`PlayerState.PlayerName` (`Controller.PlayerState` IngamePC)))))

(event `SetMenuUp`
  (params (SetMenu :type Boolean))
  (for _array_element (`/Game/Blueprints/GameplayBPs/IngameGamemode.AllPlayerControllers` (cast `/Game/Blueprints/GameplayBPs/IngameGamemode` (`GameplayStatics.GetGameMode`) :!pure true))
    (set `BaseCharacter.MenuUp` SetMenu (cast `BaseCharacter` (`Controller.K2_GetPawn` _array_element) :!pure true))))

(event `ScoreboardOn`
  (if (== (`self.RoundStarted`) false)
    (`Widget.SetVisibility` (`/Game/Blueprints/GameplayBPs/IngamePC.DuelScoreboardBP` (cast `/Game/Blueprints/GameplayBPs/IngamePC` (`GameplayStatics.GetPlayerController` 0) :!pure true)) "Visible" :!label _label)
    (set `self.ScoreboardToggled` true)))

(event `ScoreBoardOnCheck`
  (if (and (== (`self.ScoreboardToggled`) false) (== (`self.RoundStarted`) true))
    (goto _label)))

(event `ScoreboardOff`
  (`Widget.SetVisibility` (`/Game/Blueprints/GameplayBPs/IngamePC.DuelScoreboardBP` (cast `/Game/Blueprints/GameplayBPs/IngamePC` (`GameplayStatics.GetPlayerController` 0) :!pure true)) "Hidden" :!label _label_2)
  (set `self.ScoreboardToggled` false))

(event `ScoreBoardOffCheck`
  (if (and (== (`self.ScoreboardToggled`) true) (== (`self.RoundStarted`) true))
    (goto _label_2)))

(event `self.ReceiveBeginPlay`
  (`self.RoundStart`))

(event `StopAllPlayers`
  (for _array_element (`self.AllPlayerControllers`)
    (bind _asbase_character (cast `BaseCharacter` (`Controller.K2_GetPawn` _array_element) :!pure true))
    (set `BaseCharacter.Invincible` true _asbase_character)
    (set `BaseCharacter.MenuUp` true _asbase_character)))

(event `CountdownTimer`
  (set `self.StartTimer` (`KismetMathLibrary.Clamp` (- (`self.StartTimer`) 1) 0 9999))
  (if (== (`self.StartTimer`) 0)
    (set `self.RoundStarted` true)
    (`self.SetMenuUp` false)
    (`self.FightStart`)
    (bind _returnvalue (`KismetSystemLibrary.K2_SetTimer` self "RoundTimerEvent" 1.0 true))
    (set `self.RoundTimerHandle` _returnvalue)
    (`KismetSystemLibrary.K2_ClearAndInvalidateTimerHandle` (`self.RoundCountdownTimerHandle`))))

(event `RoundTimerEnded`
  (`self.StopAllPlayers`)
  (`self.FinishScored`))

(event `FightStart`
  (bind _asingame_pc (cast `/Game/Blueprints/GameplayBPs/IngamePC` (`GameplayStatics.GetPlayerController` 0) :!pure true))
  (`Widget.SetVisibility` (`/Game/Blueprints/GameplayBPs/IngamePC.DuelScoreboardBP` _asingame_pc) "Hidden")
  (set `self.ScoreboardToggled` false)
  (`/Game/Classes/Revenant/Blueprints/RevenantChooseAttacks.TimeRanOut` (`/Game/Blueprints/GameplayBPs/IngamePC.ChooseUI` _asingame_pc)))

(event `RoundStart`
  (set `self.StartTimer` 30)
  (set `self.RoundTimer` 240)
  (bind _returnvalue (`KismetSystemLibrary.K2_SetTimerDelegate` (delegate `CountdownTimer`) 1.0 true))
  (set `self.RoundCountdownTimerHandle` _returnvalue))

(event `OnScored`
  (bind _playerscorearray (`self.PlayerScoreArray`))
  (for (_array_element _array_index) _playerscorearray
    (bind (_playercontroller _score _username) (break `/Game/Blueprints/GameplayBPs/IngamePlayerScoreList` _array_element))
    (if (not (`BaseCharacter.IsDead` (cast `BaseCharacter` (`Controller.K2_GetPawn` _playercontroller) :!pure true)))
      (`KismetArrayLibrary.Array_Set` _playerscorearray _array_index (make `/Game/Blueprints/GameplayBPs/IngamePlayerScoreList` _playercontroller (+ _score 1) _username))))
  (`self.FinishScored`))

(event `FinishScored`
  (`KismetSystemLibrary.K2_ClearAndInvalidateTimerHandle` (`self.RoundTimerHandle`))
  (if (`self.RoundStarted`)
    (set `self.RoundStarted` false)
    (`self.DisplayScoreboard`)
    (`KismetSystemLibrary.Delay` 5.0)
    (`self.SetMenuUp` true)
    (set `self.RoundCount` (+ (`self.RoundCount`) 1))
    (bind (_istherewinner _winnerusername) (`self.CheckIfWinnerExists`))
    (if _istherewinner
      (`self.GameOver` _winnerusername)
      (elif (>= (`self.RoundCount`) (`self.MaxRounds`))
        (`self.ProcessWinner`)
        (else
          (`self.RoundStart`)
          (for _array_element (`/Game/Blueprints/GameplayBPs/IngameGamemode.AllPlayerControllers` (cast `/Game/Blueprints/GameplayBPs/IngameGamemode` (`GameplayStatics.GetGameMode`) :!pure true))
            (`/Game/Blueprints/GameplayBPs/IngamePC.ResetPlayers` (cast `/Game/Blueprints/GameplayBPs/IngamePC` _array_element :!pure true))))))))

(event `DisplayScoreboard`
  (`Widget.SetVisibility` (`/Game/Blueprints/GameplayBPs/IngamePC.DuelScoreboardBP` (cast `/Game/Blueprints/GameplayBPs/IngamePC` (`GameplayStatics.GetPlayerController` 0) :!pure true)) "Visible")
  (set `self.ScoreboardToggled` true))

(event `GameOver`
  (params (WinnerUsername :type String))
  (for _array_element (`self.AllPlayerControllers`)
    (`/Game/Blueprints/GameplayBPs/IngamePC.DisplayWinner` (cast `/Game/Blueprints/GameplayBPs/IngamePC` _array_element :!pure true) WinnerUsername)
    (`KismetSystemLibrary.Delay` 5.0)
    (`GameplayStatics.OpenLevel` "MainMenu")
    (`DestroySessionCallbackProxy.DestroySession` _array_element)))

(fn `CheckIfWinnerExists`
  (returns (IsThereWinner :type Boolean) (WinnerUsername :type String))
  (for _array_element (`self.PlayerScoreArray`)
    (bind (_playercontroller _score) (break `/Game/Blueprints/GameplayBPs/IngamePlayerScoreList` _array_element))
    (if (>= _score 3)
      (return true (`BaseCharacter.Username` (cast `BaseCharacter` (`Controller.K2_GetPawn` _playercontroller) :!pure true)))))
  (return false ""))

(fn `ProcessWinner`
  (bind _playerscorearray (`self.PlayerScoreArray`))
  (bind (_playercontroller _score) (break `/Game/Blueprints/GameplayBPs/IngamePlayerScoreList` (`|GetArrayItem` _playerscorearray)))
  (bind (_playercontroller_2 _score_2) (break `/Game/Blueprints/GameplayBPs/IngamePlayerScoreList` (`|GetArrayItem` _playerscorearray 1)))
  (`/Engine/EditorBlueprintResources/StandardMacros.CompareInt` _score _score_2
    (:`>`
      (`self.GameOver` (`BaseCharacter.Username` (cast `BaseCharacter` (`Controller.K2_GetPawn` _playercontroller) :!pure true))))
    (:`==`
      (`self.GameOver` "Draw!"))
    (:`<`
      (`self.GameOver` (`BaseCharacter.Username` (cast `BaseCharacter` (`Controller.K2_GetPawn` _playercontroller_2) :!pure true))))))

(fn `RoundTimerEvent`
  (set `self.RoundTimer` (`KismetMathLibrary.Clamp` (- (`self.RoundTimer`) 1) 0 9999))
  (if (<= (`self.RoundTimer`) 0)
    (`self.RoundTimerEnded`)))

(fn `UserConstructionScript`)