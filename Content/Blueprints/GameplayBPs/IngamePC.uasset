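; In-game multiplayer player controller that handles character spawning, the gameplay UI and text chat.
; On local BeginPlay it loads player settings from a save slot and passes them to the server, where MyGame respawns the chosen character, then creates chat and UI widgets.
; Chat messages fan out through the game mode's controller list to each controller's chat window.
; T toggles cursor, input mode and the pawn's MenuUp flag for chatting.
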(event `self.ReceiveBeginPlay`
  ;[1 1 1] Load Player Info and pass to Server
  (if (`self.IsLocalController`)
    (`WidgetLayoutLibrary.RemoveAllWidgets`)
    (`self.LoadGame`)
    (`self.PassCharacterInfoToServer` (`self.PlayerSettings`))))

(event `PassCharacterInfoToServer`
  (params (PlayerSettingsInfo :type "/Game/Blueprints/GameplayBPs/PlayerInfo Structure"))
  ;[1 1 1] Passes Character through Server and respawns
  (set `self.PlayerSettings` PlayerSettingsInfo)
  (bind _asmy_game (cast `/Game/Blueprints/GameplayBPs/MyGame` (`GameplayStatics.GetGameMode`)))
  (`/Game/Blueprints/GameplayBPs/MyGame.Respawn Player` _asmy_game self (`.MyPlayerCharacter_9_96D4F7F747878F18E4BFF386343EEB3C` (break `/Game/Blueprints/GameplayBPs/PlayerInfo` (`self.PlayerSettings`))))
  (`self.SetupChatWindow`))

(event `SetupChatWindow`
  ;[1 1 1] Creates GameChat
  (`WidgetLayoutLibrary.RemoveAllWidgets`)
  (bind _returnvalue (`|CreateWidget` "/Game/Menus/Chat/GameplayChat.GameplayChat_C"))
  (bind _output_get (set `self.GameplayChatWB` _returnvalue))
  (`UserWidget.AddToViewport` _output_get 0)
  (bind _returnvalue_2 (`|CreateWidget` "/Game/Menus/IngameUI/UI.UI_C"))
  (`UserWidget.AddToViewport` _returnvalue_2 0))

(event `GetChatMessage`
  (params (`Text to Send` :type Text))
  ;[1 1 1] Process Chat
  (set `self.Sender Text` `Text to Send`)
  (set `self.SenderName` (`.MyPlayerName_2_F5939672454D9B3A86D19BB0E97B5861` (break `/Game/Blueprints/GameplayBPs/PlayerInfo` (`self.PlayerSettings`))))
  (bind _asmy_game (cast `/Game/Blueprints/GameplayBPs/MyGame` (`GameplayStatics.GetGameMode`)))
  (for _array_element (`/Game/Blueprints/GameplayBPs/MyGame.AllPlayerControllers` _asmy_game)
    (bind _asingame_pc (cast `/Game/Blueprints/GameplayBPs/IngamePC` _array_element))
    (`self.UpdateChat` _asingame_pc (`self.SenderName`) (`self.Sender Text`))))

(event `Key|T`
  (params (Key :type "Key Structure"))
  (:`Pressed`
    (`/Engine/EditorBlueprintResources/StandardMacros.FlipFlop`
      (:`A`
        (set `self.bShowMouseCursor` true)
        (`WidgetBlueprintLibrary.SetInputMode_GameAndUIEx` self (`self.GameplayChatWB`))
        (set `BaseCharacter.MenuUp` true (cast `BaseCharacter` (`self.K2_GetPawn`) :!pure true)))
      (:`B`
        (set `self.bShowMouseCursor` false)
        (`WidgetBlueprintLibrary.SetInputMode_GameOnly` self)
        (set `BaseCharacter.MenuUp` false (cast `BaseCharacter` (`self.K2_GetPawn`) :!pure true))))))

(event `UpdateChat`
  (params (SenderName :type Text) (SenderText :type Text))
  ;[1 1 1] Update Client Chat
  (`/Game/Menus/Chat/ChatWindow.UpdateChatWindow` (`/Game/Menus/Chat/GameplayChat.GameChat` (`self.GameplayChatWB`)) SenderName SenderText))

(fn `LoadGame`
  (bind _returnvalue (`GameplayStatics.LoadGameFromSlot` (`self.PlayerSettingSave`)))
  (bind _asplayer_save_info (cast `/Game/Blueprints/GameplayBPs/PlayerSaveInfo` _returnvalue))
  (set `self.PlayerSettings` (`/Game/Blueprints/GameplayBPs/PlayerSaveInfo.S_PlayerInfo` _asplayer_save_info)))

(fn `UserConstructionScript`)